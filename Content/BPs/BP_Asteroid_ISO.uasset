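; Asteroid actor for the asteroid simulator, pulled toward the game mode's Earth by Newtonian gravity and sized from StartRadius at construction.
; Each Tick scales delta time by TimeMultiplier, then moves with sweep, updates Velocity, and recomputes inverse-square acceleration from G and Earth's mass.
; This explicit Euler-style step applies each new acceleration on the following frame.
; StartSpeed only seeds CurrentSpeed, which movement does not read.
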(event EventBeginPlay
  (bind _asbp_asteroid_simulator_gm (Utilities|Casting|CastToBP_AsteroidSimulatorGM (Game|GetGameMode)))
  (Variables|Default|SetAsteroidSimulatorGameMode _asbp_asteroid_simulator_gm)
  (Variables|Default|SetcurrentSpeed (Variables|Default|GetstartSpeed))
  (Variables|Default|SetcurrentAcceleration "0, 0, 0")
  (Variables|Default|SetcurrentRadius (Variables|Default|GetstartRadius)))

(event EventTick
  (params (DeltaSeconds :type Float%20%28single-precision%29))
  (bind _asteroidsimulatorgamemode (Variables|Default|GetAsteroidSimulatorGameMode))
  (bind _timemultiplier (Variables|/Game/BPs/BP_AsteroidSimulatorGM.BP_AsteroidSimulatorGM_C|GettimeMultiplier _asteroidsimulatorgamemode))
  (bind _returnvalue (* DeltaSeconds _timemultiplier))
  (CallFunction|Move _returnvalue)
  (CallFunction|Accelerate _returnvalue)
  (CallFunction|ApplyGravityForce _returnvalue))

(fn ConstructionScript
  (Transformation|SetRelativeScale3D (Variables|Default|GetStaticMesh) (Math|Conversions|ToVector(Float) (* (Variables|Default|GetstartRadius) 2.0))))

(fn Move
  (params (deltaTime :type Float%20%28single-precision%29))
  (Transformation|AddActorWorldOffset (* (Variables|Default|Getvelocity) deltaTime) true))

(fn Accelerate
  (params (deltaTime :type Float%20%28single-precision%29))
  (Variables|Default|Setvelocity (+ (Variables|Default|Getvelocity) (* (Variables|Default|GetcurrentAcceleration) deltaTime))))

(fn ApplyGravityForce
  (params (deltaTime :type Float%20%28single-precision%29))
  (bind _returnvalue (Transformation|GetActorLocation))
  (bind _asteroidsimulatorgamemode (Variables|Default|GetAsteroidSimulatorGameMode))
  (bind _earth (Variables|/Game/BPs/BP_AsteroidSimulatorGM.BP_AsteroidSimulatorGM_C|GetEarth _asteroidsimulatorgamemode))
  (bind _returnvalue_2 (Transformation|GetActorLocation _earth))
  (bind _returnvalue_3 (- _returnvalue_2 _returnvalue))
  (Variables|Default|SetcurrentAcceleration (* (Math|Vector|Normalize _returnvalue_3) (/ (* 1.0 (Variables|/Game/BPs/BP_AsteroidSimulatorGM.BP_AsteroidSimulatorGM_C|GetG _asteroidsimulatorgamemode) (Variables|/Game/BPs/BP_Earth.BP_Earth_C|GetMass _earth)) (Math|Vector|VectorLengthSquared _returnvalue_3)))))