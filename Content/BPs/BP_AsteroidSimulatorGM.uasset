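; Game mode for the asteroid simulator that handles the in-game pause menu.
; On BeginPlay it enables input on itself for the first player controller and creates the menu widget once.
; The InGameMenu input action calls ToggleInGameMenu, which adds or removes that widget, shows or hides the mouse cursor, and pauses or resumes the game.
; A SetGlobalTimeDilation node is left unconnected and never runs.
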(event EventBeginPlay
  (Input|EnableInput (Game|GetPlayerController 0))
  (bind _returnvalue (UserInterface|CreateWidget "/Game/UI/InGameMenu_WidgetBlueprint.InGameMenu_WidgetBlueprint_C"))
  (Variables|Default|SetInGameMenuWidget _returnvalue))

(event Input|ActionEvents|InputActionInGameMenu
  (params (Key :type Key%20Structure :default "AnyKey"))
  (:Pressed
    (CallFunction|ToggleinGameMenu (not (UserInterface|Viewport|IsinViewport (Variables|Default|GetInGameMenuWidget))))))

(fn ConstructionScript)

(fn ToggleinGameMenu
  (params (enable :type Boolean))
  (bind _returnvalue (Game|GetPlayerController 0))
  (bind _ingamemenuwidget (Variables|Default|GetInGameMenuWidget))
  (bind _returnvalue_2 (UserInterface|Viewport|IsinViewport _ingamemenuwidget))
  (if enable
    (if (not _returnvalue_2)
      (UserInterface|Viewport|AddtoViewport _ingamemenuwidget 0)
      (Variables|/Script/Engine.PlayerController|SetbShowMouseCursor _returnvalue true)
      (Game|SetGamePaused true))
    (elif _returnvalue_2
      (Widget|RemovefromParent _ingamemenuwidget)
      (Variables|/Script/Engine.PlayerController|SetbShowMouseCursor _returnvalue false)
      (Game|SetGamePaused false))))